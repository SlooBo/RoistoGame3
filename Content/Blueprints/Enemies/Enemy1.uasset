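; Enemy1 is a simple enemy actor that chases the player and destroys itself when its health runs out.
; Each Tick it snaps its rotation to face player pawn 0, then moves a fixed step along its forward vector with vertical movement zeroed.
; Movement is unswept and not scaled by delta time, so speed depends on frame rate.
; The same Tick polls Health for death; nothing in this graph changes that value.
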(event EventBeginPlay)

(event EventActorBeginOverlap
  (params (OtherActor :type Actor%20Object%20Reference)))

(event EventTick
  (params (DeltaSeconds :type Float%20%28single-precision%29))
  (bind _returnvalue (Transformation|GetActorRotation))
  (bind _returnvalue_2 (Math|Vector|GetForwardVector _returnvalue))
  (bind _returnvalue_3 (* _returnvalue_2 5.0))
  (bind (_x _y) (Math|Vector|BreakVector _returnvalue_3))
  (Transformation|SetActorRotation (Math|Rotator|FindLookatRotation (Transformation|GetActorLocation) (Transformation|GetActorLocation (Game|Player|GetPlayerPawn 0))))
  (Transformation|AddActorWorldOffset (Math|Vector|MakeVector _x _y 0.0))
  (if (<= (Variables|Default|GetHealth) 0.0)
    (Actor|DestroyActor)))

(fn ConstructionScript
  (|CallParentFunction))