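; Player pawn for a top-down shooter, with axis movement, mouse-cursor aiming, health and knockback.
; Tick rotates the pawn's Empty component toward the cursor, drives delayed health regen and plays step sounds on movement.
; Holding left mouse opens a gate that fires delay-paced bullets along the aim, with MultiShotAmount adding angled extras.
; AddSawBlade attaches up to eight sawblade weapons at slot positions on a constantly spinning SawBlades component.
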(event EventBeginPlay
  (Variables|/Script/Engine.PlayerController|SetbShowMouseCursor (Game|GetPlayerController 0) true))

(event EventActorBeginOverlap
  (params (OtherActor :type Actor%20Object%20Reference)))

(event EventTick
  (params (DeltaSeconds :type Float%20%28single-precision%29))
  (bind _returnvalue (Transformation|GetActorLocation))
  (CallFunction|RotatePlayer)
  (Utilities|FlowControl|Sequence
    (:then_0
      (CallFunction|CheckHealth)
      (Utilities|FlowControl|Delay (Variables|Default|GetHpRegenDelay))
      (CallFunction|RegenHealth))
    (:then_1
      ;[1 1 1] Shoot
      (Utilities|FlowControl|Gate true
        (:Exit
          (Utilities|FlowControl|Delay (Variables|Default|GetAttackSpeed))
          (CallFunction|Shoot))))
    (:then_2
      (CallFunction|RotateSawBlades))
    (:then_3
      (Utilities|FlowControl|Delay 0.5)
      (Variables|Default|SetLastLocation _returnvalue))
    (:then_4
      (Utilities|FlowControl|Delay 0.3)
      (if (not (Math|Vector|Equal(Vector) _returnvalue (Variables|Default|GetLastLocation) 1.0))
        (Audio|PlaySoundatLocation "/Game/Audio/Effects/Step.Step" "0, 0, 0" "0, 0, 0" 0.3)))))

(event Input|ActionEvents|InputActionActionLeftMouse
  (params (Key :type Key%20Structure :default "AnyKey"))
  ;[1 1 1] Shoot
  (:Pressed
    (Utilities|FlowControl|Gate true) ; enters at Open
  )
  (:Released
    (Utilities|FlowControl|Gate true) ; enters at Close
  ))

(event Input|AxisEvents|InputAxisAxisForward
  (params (AxisValue :type Float%20%28single-precision%29))
  ;[1 1 1] Movement
  (Pawn|Input|AddMovementInput (Pawn|GetControlledPawn (Game|GetPlayerController 0)) (Math|Vector|MakeVector (Variables|Default|GetMoveSpeed) 0.0 0.0) AxisValue false))

(event Input|AxisEvents|InputAxisAxisRight
  (params (AxisValue :type Float%20%28single-precision%29))
  ;[1 1 1] Movement
  (Pawn|Input|AddMovementInput (Pawn|GetControlledPawn (Game|GetPlayerController 0)) (Math|Vector|MakeVector 0.0 (Variables|Default|GetMoveSpeed) 0.0) AxisValue false))

(fn ConstructionScript)

(fn RotatePlayer
  (bind _returnvalue (Game|GetPlayerController 0))
  (bind _empty (Variables|Default|Getempty))
  (bind _worldlocation (Game|Player|ConvertMouseLocationToWorldSpace _returnvalue))
  (bind _returnvalue_2 (Transformation|GetWorldLocation _empty))
  (bind (_x _y) (Math|Vector|BreakVector _returnvalue_2))
  (bind (_x_2 _y_2) (Math|Vector|BreakVector _worldlocation))
  (bind _returnvalue_3 (Math|Vector|MakeVector _x _y 0.0))
  (bind _returnvalue_4 (Math|Vector|MakeVector _x_2 _y_2 0.0))
  (bind _returnvalue_5 (Math|Rotator|FindLookatRotation _returnvalue_3 _returnvalue_4))
  (Transformation|SetWorldRotation (Variables|Default|Getempty) _returnvalue_5 false false)
  (Variables|Default|SetLookAtRot _returnvalue_5))

(fn Shoot
  (bind _returnvalue (Transformation|GetActorLocation))
  (bind _returnvalue_2 (Transformation|GetActorLocation))
  (bind _lookatrot (Variables|Default|GetLookAtRot))
  (bind _lookatrot_2 (Variables|Default|GetLookAtRot))
  (bind (_roll _pitch _yaw) (Math|Rotator|BreakRotator _lookatrot))
  (bind (_roll_2 _pitch_2 _yaw_2) (Math|Rotator|BreakRotator _lookatrot_2))
  (Game|SpawnActorfromClass "/Game/Blueprints/Weapons/Bullet.Bullet_C" (Math|Transform|MakeTransform (Transformation|GetActorLocation) (Variables|Default|GetLookAtRot)) "Undefined" 0 0)
  (Utilities|FlowControl|Sequence
    (:then_0
      ;[1 1 1] Multishot
      (if (not (<= (Variables|Default|GetMultiShotAmount) 0))
        (Game|SpawnActorfromClass "/Game/Blueprints/Weapons/Bullet.Bullet_C" (Math|Transform|MakeTransform _returnvalue_2 (Math|Rotator|MakeRotator _roll_2 _pitch_2 (+ _yaw_2 7.0))) "Undefined" 0 0)
        (if (not (<= (Variables|Default|GetMultiShotAmount) 1))
          (Game|SpawnActorfromClass "/Game/Blueprints/Weapons/Bullet.Bullet_C" (Math|Transform|MakeTransform _returnvalue_2 (Math|Rotator|MakeRotator _roll_2 _pitch_2 (+ _yaw_2 -7.0))) "Undefined" 0 0)
          (if (not (<= (Variables|Default|GetMultiShotAmount) 2))
            (Game|SpawnActorfromClass "/Game/Blueprints/Weapons/Bullet.Bullet_C" (Math|Transform|MakeTransform _returnvalue (Math|Rotator|MakeRotator _roll _pitch (+ _yaw 13.0))) "Undefined" 0 0)
            (if (not (<= (Variables|Default|GetMultiShotAmount) 3))
              (Game|SpawnActorfromClass "/Game/Blueprints/Weapons/Bullet.Bullet_C" (Math|Transform|MakeTransform _returnvalue (Math|Rotator|MakeRotator _roll _pitch (+ _yaw -13.0))) "Undefined" 0 0))))))
    (:then_1
      (Audio|PlaySoundatLocation "/Game/Audio/Effects/Dash.Dash" (Transformation|GetActorLocation)))))

(fn RotateSawBlades
  (Transformation|AddLocalRotation (Variables|Default|GetSawBlades) "0,5.000000, 0" false false))

(fn AddSawBlade
  (Variables|Default|SetSawBladeAmount (+ (Variables|Default|GetSawBladeAmount) 1))
  (switch int (Variables|Default|GetSawBladeAmount)
    (:1
      (Variables|Default|SetSawbladeTransform (Math|Transform|MakeTransform (Transformation|GetWorldLocation (Variables|Default|GetSlot1)) "0, 0, 0" "0.300000,0.300000,0.300000")))
    (:2
      (Variables|Default|SetSawbladeTransform (Math|Transform|MakeTransform (Transformation|GetWorldLocation (Variables|Default|GetSlot2)) "0, 0, 0" "0.300000,0.300000,0.300000")))
    (:3
      (Variables|Default|SetSawbladeTransform (Math|Transform|MakeTransform (Transformation|GetWorldLocation (Variables|Default|GetSlot3)) "0, 0, 0" "0.300000,0.300000,0.300000")))
    (:4
      (Variables|Default|SetSawbladeTransform (Math|Transform|MakeTransform (Transformation|GetWorldLocation (Variables|Default|GetSlot4)) "0, 0, 0" "0.300000,0.300000,0.300000")))
    (:5
      (Variables|Default|SetSawbladeTransform (Math|Transform|MakeTransform (Transformation|GetWorldLocation (Variables|Default|GetSlot5)) "0, 0, 0" "0.300000,0.300000,0.300000")))
    (:6
      (Variables|Default|SetSawbladeTransform (Math|Transform|MakeTransform (Transformation|GetWorldLocation (Variables|Default|GetSlot6)) "0, 0, 0" "0.300000,0.300000,0.300000")))
    (:7
      (Variables|Default|SetSawbladeTransform (Math|Transform|MakeTransform (Transformation|GetWorldLocation (Variables|Default|GetSlot7)) "0, 0, 0" "0.300000,0.300000,0.300000")))
    (:8
      (Variables|Default|SetSawbladeTransform (Math|Transform|MakeTransform (Transformation|GetWorldLocation (Variables|Default|GetSlot8)) "0, 0, 0" "0.300000,0.300000,0.300000"))))
  (bind _returnvalue (Game|SpawnActorfromClass "/Game/Blueprints/Weapons/Weapon_Sawblade.Weapon_Sawblade_C" (Variables|Default|GetSawbladeTransform) "Undefined" 0 0))
  (Class|Actor|AttachRootComponentto _returnvalue (Variables|Default|GetSawBlades) "None" "KeepWorldPosition" true))

(fn CheckHealth
  (if (<= (Variables|Default|GetHealth) 0.0)
    (Variables|Default|SetAlive false)))

(fn RegenHealth
  (Variables|Default|SetHealth (+ (Variables|Default|GetHealth) 0.1)))

(fn TakeDamage
  (params (damageamount :type Float%20%28single-precision%29) (knockback :type Boolean) (knockbackdir :type Vector) (knockbackamount :type Float%20%28single-precision%29))
  (if knockback
    (CallFunction|Knockback knockbackdir knockbackamount))
  (Variables|Default|SetHealth (- (Variables|Default|GetHealth) damageamount))
  (Development|PrintString (Utilities|String|ToString(Float) (Variables|Default|GetHealth))))

(fn Knockback
  (params (direction :type Vector) (amount :type Float%20%28single-precision%29))
  (Transformation|AddActorWorldOffset (* direction amount)))